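; Flame pillar actor that makes its fire light flicker continuously.
; On BeginPlay it randomly picks one of two intensity timelines and plays it from the start, choosing again whenever one finishes.
; Each timeline update feeds ScaleFireIntensity, which multiplies the curve value by BaseIntensity to set the FireLight intensity, so the flicker pattern varies over time.
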(event Custom|StartTimeLine_2
  (bind _firteintensity_1 (Timeline|FirteIntensityTimeline_2 PlayFromStart)
    (:Update
      (CallFunction|ScaleFireIntensity _firteintensity_1))
    (:Finished
      (CallFunction|ChooseFire))))

(event Custom|StartTimeLine_1
  (bind _firteintensity_0 (Timeline|FirteIntensityTimeline_1 PlayFromStart)
    (:Update
      (CallFunction|ScaleFireIntensity _firteintensity_0))
    (:Finished
      (CallFunction|ChooseFire))))

(event Custom|ChooseFire
  (switch int (Math|Random|RandomIntegerinRange 0 1)
    (:Default
      (CallFunction|StartTimeLine2 :!label _label))
    (:0
      (CallFunction|StartTimeLine1))
    (:1
      (goto _label))))

(event EventBeginPlay
  (CallFunction|ChooseFire))

(fn ConstructionScript)

(fn ScaleFireIntensity
  (params (Intensity :type Float%20%28double-precision%29))
  (Rendering|Components|Light|SetIntensity (Variables|Default|GetFireLight) (* Intensity (Variables|Default|GetBaseIntensity))))