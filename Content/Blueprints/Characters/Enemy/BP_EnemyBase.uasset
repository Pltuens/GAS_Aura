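; Base enemy character Blueprint that handles spawn scale-in, death-style dissolve effects and loot drops.
; Timelines drive the mesh scale on BeginPlay and the Dissolve parameter on body and weapon dynamic materials.
; SpawnLoot pulls items from loot tiers, then a looping timer spawns them one by one at evenly spaced directions and random distances, passing enemy level to AuraEffectActors.
; A Motion Warping target named FacingTarget updates from a supplied location.
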(event Custom|SpawnLootItem
  (bind _lootitems (Variables|Default|GetLootItems))
  (bind _spawnlootcount (Variables|Default|GetSpawnLootCount))
  (bind _output (Utilities|Array|Get(acopy) _lootitems _spawnlootcount))
  (bind (_lootclass _blootleveloverride) (Utilities|Struct|BreakLootItem _output))
  (if (< (Variables|Default|GetSpawnLootCount) (Utilities|Array|Length (Variables|Default|GetLootItems)))
    (bind _returnvalue (Game|SpawnActorfromClass _lootclass (CallFunction|GetLootTransForm (Variables|Default|GetSpawnLootCount)) "AlwaysSpawn" "MultiplyWithRoot" 0 0))
    (bind _asaura_effect_actor (Utilities|Casting|CastToAuraEffectActor _returnvalue)
      (:then
        (Variables|/Script/GAS_Aura.AuraEffectActor|SetActorLevel _asaura_effect_actor (Math|Conversions|ToFloat(Integer) (Variables|Default|GetLevel)))
        (if _blootleveloverride
          _
          (else
            _)))
      (:CastFailed
        _))
    (Math|Integer|IncrementInt (Variables|Default|GetSpawnLootCount))
    (else
      (Utilities|Time|ClearandInvalidateTimerbyHandle (Variables|Default|GetLootTimer)))))

(event EventBeginPlay
  (bind _scaletrack (Timeline|SpawnTimeline Play)
    (:Update
      (Transformation|SetRelativeScale3D (Variables|Character|GetMesh) (Math|Vector|MakeVector _scaletrack _scaletrack _scaletrack)))))

(event EventSpawnLoot
  (bind _returnvalue (Class|AuraAbilitySystemLibrary|GetLootTiers))
  (Utilities|IsValid _returnvalue
    (:Is%20Valid
      (bind _returnvalue_2 (Class|LootTiers|GetLootItems _returnvalue))
      (bind _output_get (Variables|Default|SetLootItems _returnvalue_2))
      (Variables|Default|SetLoot%20Rotations (CallFunction|GetLootRotations _output_get))
      (Variables|Default|SetSpawnLootCount 0)
      (bind _returnvalue_3 (Utilities|Time|SetTimerbyEvent (delegate Custom|SpawnLootItem) 0.1 true))
      (Variables|Default|SetLootTimer _returnvalue_3)
      (CallFunction|SpawnLootItem))))

(event EventStartDissolveTimeline
  (params (MaterialInstanceDynamic :type Material%20Instance%20Dynamic%20Object%20Reference))
  (bind _溶解轨道 (Timeline|溶解%20%20时间轴 Play)
    (:Update
      (Rendering|Material|SetScalarParameterValue MaterialInstanceDynamic "Dissolve" _溶解轨道 :!class /Script/Engine.MaterialInstanceDynamic))))

(event EventStartWeaponDissolveTimeline
  (params (MaterialInstanceDynamic :type Material%20Instance%20Dynamic%20Object%20Reference))
  (bind _武器溶解_轨道 (Timeline|武器溶解 Play)
    (:Update
      (Rendering|Material|SetScalarParameterValue MaterialInstanceDynamic "Dissolve" _武器溶解_轨道 :!class /Script/Engine.MaterialInstanceDynamic))))

(event EventUpdateFacingTarget
  (params (FacingTarget :type Vector%20%28by%20ref%29 :default "0, 0, 0"))
  (Class|MotionWarpingComponent|AddorUpdateWarpTargetfromLocation (Variables|Default|GetMotionWarping) "FacingTarget" FacingTarget))

(fn ConstructionScript)

(fn GetLootRotations
  (params (TargetArray :type Array%20of%20Loot%20Item%20Structures))
  (return (Class|AuraAbilitySystemLibrary|EvenlySpacedRotators (Transformation|GetActorForwardVector) (Math|Vector|VectorUp) 3.6e+02 (Utilities|Array|Length TargetArray))))

(fn GetLootTransForm
  (params (LootCount :type Integer))
  (bind _loot_rotations (Variables|Default|GetLoot%20Rotations))
  (bind _output (Utilities|Array|Get(acopy) _loot_rotations LootCount))
  (return (Math|Transform|MakeTransform (+ (* (Math|Vector|GetForwardVector _output) (Math|Random|RandomFloatinRange (LocalVariables|GetMinSpawnDistance) (LocalVariables|GetMaxSpawnDistance))) (Transformation|GetActorLocation)) _output)))